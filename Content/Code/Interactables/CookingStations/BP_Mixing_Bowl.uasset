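; BP_Mixing_Bowl is an interactable cooking station that shows batter when it holds items and animates a spoon during its minigame.
; Minigame start readies the spoon animation, and finishing stops it before passing quality to the parent.
; Inventory updates count filled slots to set or clear the Filler's batter mesh.
; The inventory-update binding is made on Tick rather than BeginPlay.
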(event `self.ReceiveBeginPlay`
  (add `self.MiniGameStart` (delegate `CallAnimation`)))

(event `CallAnimation`
  (`/Game/Code/Interactables/BP_Spoon_MixingBowl.ReadyAnimation` (`self.Spoon`)))

(event `self.ReceiveTick`
  (params (DeltaSeconds :type "Float (single-precision)"))
  (add `/Game/Code/Core/Inventory/BP_InventorySystem.OnInventoryUpdated` (`self.BP_InventorySystem`) (delegate `UpdateDisplay`)))

(event `UpdateDisplay`
  (`self.CheckIfNotEmpty`))

(fn `CheckIfNotEmpty`
  (`|ExecutionSequence`
    (:`then_0`
      (set `self.LocalCounter` 0)
      (for _array_element (`/Game/Code/Core/Inventory/BP_InventorySystem.Content` (`self.BP_InventorySystem`))
        (if (> (`.Quantity_5_614ED38643097AB082B4D6BD820F5592` (break `/Game/Code/Core/Inventory/FSlotStruct` _array_element)) 0)
          (`/Engine/EditorBlueprintResources/StandardMacros.IncrementInt` (`self.LocalCounter`)))))
    (:`then_1`
      (if (> (`self.LocalCounter`) 0)
        (`self.DisplayItems`)
        (else
          (`self.RemoveDisplayedItem`))))))

(fn `DisplayItems`
  (bind _returnvalue (`StaticMeshComponent.SetStaticMesh` (`self.Filler`) "/Game/Art/1-Assets/Ingredients/PotAndBowlFiller/SM_Batter.SM_Batter"))
  (set `self.MeshDisplayed` _returnvalue))

(fn `LookAtBackup`
  (returns (Message :type Text))
  (return ""))

(fn `OnMinigameFinished`
  (params (Quality :type "Float (double-precision)"))
  (`/Game/Code/Interactables/BP_Spoon_MixingBowl.StopAnimation` (`self.Spoon`))
  (`parent.OnMinigameFinished` Quality))

(fn `RemoveDisplayedItem`
  (`StaticMeshComponent.SetStaticMesh` (`self.Filler`) null)
  (set `self.MeshDisplayed` false))

(fn `UserConstructionScript`)