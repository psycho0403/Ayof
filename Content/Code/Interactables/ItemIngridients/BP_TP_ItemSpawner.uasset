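; BP_TP_ItemSpawner is an ingredient spawner that keeps track of one current item at its location.
; On BeginPlay it spawns the ItemsToSpawn entry matching TypeOfIngredient, with itself as owner, and stores the sprite's Y position.
; AttemptSpawn skips spawning while CurrentItem is valid.
; The Respawn event clears that reference and spawns a replacement after a short delay.
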(event `self.ReceiveBeginPlay`
  (bind (_returnvalue_x _returnvalue_y) (`KismetMathLibrary.BreakVector` (`SceneComponent.K2_GetComponentLocation` (`self.SpriteComponent`))))
  (`self.AttemptSpawn`)
  (set `self.ItemYPos` _returnvalue_y))

(event `/Game/Code/Interactables/ItemIngridients/BPI_ItemSpawner.Respawn`
  (set `self.CurrentItem` null)
  (`KismetSystemLibrary.Delay` 1.0)
  (`self.AttemptSpawn`))

(fn `AttemptSpawn`
  (`/Engine/EditorBlueprintResources/StandardMacros.IsValid` (`self.CurrentItem`)
    (:`Is Valid`
      (`KismetSystemLibrary.PrintString` "ItemAlreadySpawned"))
    (:`Is Not Valid`
      (`self.SpawnItem`))))

(fn `SpawnItem`
  (locals (NewLocalVar :type Integer))
  (for (_array_element _array_index) (`self.ItemsToSpawn`)
    (if (== _array_element (`self.TypeOfIngredient`))
      (bind _output_get (set `local.NewLocalVar` _array_index))
      (bind _returnvalue (`|SpawnActorFromClass` (`|GetArrayItem` (`self.ItemsToSpawn`) _output_get) (`KismetMathLibrary.MakeTransform` (`self.K2_GetActorLocation`) (`self.K2_GetActorRotation`)) "AdjustIfPossibleButAlwaysSpawn" "MultiplyWithRoot" self 0.0 null))
      (set `self.CurrentItem` _returnvalue))))

(fn `UserConstructionScript`)