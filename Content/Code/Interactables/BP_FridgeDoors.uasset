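; Interactable fridge whose upper and lower doors swing open and closed together when a player interacts with it.
; OnInteract toggles a FlipFlop that plays or reverses a timeline, lerping both doors' yaw, then calls the parent.
; A MetaSound attached at BeginPlay receives Open and Close triggers through a validity-checked helper.
; LookAt returns a name as the message text.
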(event `self.ReceiveBeginPlay`
  (bind _returnvalue (`GameplayStatics.SpawnSoundAttached` "/Game/Audio/MetaSounds/SFX/MS_Fridge.MS_Fridge" (`self.DefaultSceneRoot`) "None" (0.0 0.0 0.0) (struct) "KeepRelativeOffset" false 1.0 1.0 0.0 null null))
  (set `self.SoundComponent` _returnvalue))

(event `Open&Close`
  (`/Engine/EditorBlueprintResources/StandardMacros.FlipFlop`
    (:`A`
      (`self.SafeTriggerSound` (`self.SoundComponent`) "Open")
      (bind (_direction _doorrotation) (`Timeline|DoorTimeLine` :!label _label)
        (:`Update`
          (`SceneComponent.K2_SetRelativeRotation` (`self.LowerDoor`) (`KismetMathLibrary.MakeRotator` 0.0 0.0 (`KismetMathLibrary.Lerp` 0.0 -120.0 _doorrotation)) false false)
          (`SceneComponent.K2_SetRelativeRotation` (`self.UpperDoor`) (`KismetMathLibrary.MakeRotator` 0.0 0.0 (`KismetMathLibrary.Lerp` 0.0 -120.0 _doorrotation)) false false))))
    (:`B`
      (`self.SafeTriggerSound` (`self.SoundComponent`) "Close")
      (goto _label :!via `Reverse`))))

(fn `LookAt`
  (returns (Message :type Text) (SM :type "StaticMeshComponent Object Reference"))
  (return (`KismetTextLibrary.Conv_NameToText` (`self.Name`)) null))

(fn `OnInteract`
  (params (interactingPlayer :type "MyPlayerController Object Reference"))
  (`self.Open&Close`)
  (`parent.OnInteract` interactingPlayer))

(fn `SafeTriggerSound`
  (params (AudioComponent :type "AudioComponent Object Reference") (TriggerName :type Name))
  (`/Engine/EditorBlueprintResources/StandardMacros.IsValid` AudioComponent
    (:`Is Valid`
      (`AudioParameterControllerInterface.SetTriggerParameter` AudioComponent TriggerName))))

(fn `UserConstructionScript`)