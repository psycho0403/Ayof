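; Spoon interactable for the cooking pot, an animated skeletal mesh controlled through three functions, with no active event graph logic.
; ReadyAnimation moves the root to a hard-coded relative transform and starts then immediately stops the spoon animation.
; TriggerAnimation plays it once and broadcasts AnimationTriggered.
; StopAnimation rewinds the animation and sets another hard-coded, tilted transform; the old mixing sound calls are disconnected.
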(fn `ReadyAnimation`
  (bind _skeletalmesh (`self.SkeletalMesh`))
  (`SceneComponent.K2_SetRelativeTransform` (`self.DefaultSceneRoot`) (`KismetMathLibrary.MakeTransform` (-714.0 108.0 126.0)) false false)
  (`SkeletalMeshComponent.PlayAnimation` _skeletalmesh "/Game/Art/1-Assets/Decorations/Animated/Spoon_Anim/SKM_Spoon_Interactable_Anim.SKM_Spoon_Interactable_Anim" false)
  (`SkeletalMeshComponent.Stop` _skeletalmesh))

(fn `StopAnimation`
  (bind _skeletalmesh (`self.SkeletalMesh`))
  (`SkeletalMeshComponent.Stop` _skeletalmesh)
  (`SkeletalMeshComponent.SetPosition` _skeletalmesh 0.0 false)
  (`SceneComponent.K2_SetRelativeTransform` (`self.DefaultSceneRoot`) (`KismetMathLibrary.MakeTransform` (-714.0 97.0 140.0) (struct :`Yaw` -180.0 :`Roll` -46.0)) false false))

(fn `TriggerAnimation`
  (`SkeletalMeshComponent.PlayAnimation` (`self.SkeletalMesh`) "/Game/Art/1-Assets/Decorations/Animated/Spoon_Anim/SKM_Spoon_Interactable_Anim.SKM_Spoon_Interactable_Anim" false)
  (`self.AnimationTriggered`))

(fn `UserConstructionScript`)