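; BP_Drawer is an interactable drawer that toggles open and closed when a player interacts with it.
; A FlipFlop plays or reverses a timeline sliding the drawer along relative Y, while an attached MetaSound fires its Open trigger on each toggle.
; The same timeline moves the linked Spawner and any valid spawned item along world Y, so contents travel with the drawer.
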(event `Open&Close`
  (bind _spawner (`self.Spawner`))
  (bind _rootcomponent (`Actor.RootComponent` _spawner))
  (bind _currentitem (`/Game/Code/Interactables/ItemIngridients/BP_TP_ItemSpawner.CurrentItem` _spawner))
  (bind _itemypos (`/Game/Code/Interactables/ItemIngridients/BP_TP_ItemSpawner.ItemYPos` _spawner))
  (bind (_returnvalue_x _returnvalue_y _returnvalue_z) (`KismetMathLibrary.BreakVector` (`SceneComponent.K2_GetComponentLocation` _rootcomponent)))
  (bind _returnvalue (`GameplayStatics.SpawnSoundAttached` "/Game/Audio/MetaSounds/SFX/MS_GenericOpenClose.MS_GenericOpenClose" (`self.DefaultSceneRoot`) "None" (0.0 0.0 0.0) (struct) "KeepRelativeOffset" false 1.0 1.0 0.0 null null))
  (bind _output_get (set `self.AudioComponent` _returnvalue))
  (`AudioParameterControllerInterface.SetTriggerParameter` _output_get "Open")
  (`/Engine/EditorBlueprintResources/StandardMacros.FlipFlop`
    (:`A`
      (bind (_direction _newtrack_0) (`Timeline|Drawer Slide` :!label _label)
        (:`Update`
          (`SceneComponent.K2_SetRelativeLocation` (`self.Drawer`) (`KismetMathLibrary.MakeVector` 0.0 (`KismetMathLibrary.Lerp` 0.0 40.0 _newtrack_0)) false false)
          (bind _returnvalue_2 (`KismetMathLibrary.Lerp` _itemypos (+ _itemypos 40.0) _newtrack_0))
          (`SceneComponent.K2_SetWorldLocation` _rootcomponent (`KismetMathLibrary.MakeVector` _returnvalue_x _returnvalue_2 _returnvalue_z) false false)
          (`/Engine/EditorBlueprintResources/StandardMacros.IsValid` _currentitem
            (:`Is Valid`
              (`SceneComponent.K2_SetWorldLocation` (`Actor.RootComponent` _currentitem) (`KismetMathLibrary.MakeVector` _returnvalue_x _returnvalue_2 _returnvalue_z) false false))))))
    (:`B`
      (goto _label :!via `Reverse`))))

(fn `LookAt`
  (returns (Message :type Text) (SM :type "StaticMeshComponent Object Reference"))
  (return (`KismetTextLibrary.Conv_NameToText` (`self.Name`)) null))

(fn `OnInteract`
  (params (interactingPlayer :type "MyPlayerController Object Reference"))
  (`self.Open&Close`)
  (`parent.OnInteract` interactingPlayer))

(fn `UserConstructionScript`)